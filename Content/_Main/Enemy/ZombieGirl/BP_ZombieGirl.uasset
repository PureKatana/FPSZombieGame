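; BP_ZombieGirl is a zombie enemy that chases and melees the first-person player.
; Pawn sensing and point damage set SeePlayer on the AI blackboard, with sighting also raising walk speed.
; Attack uses a montage notify to sphere-overlap at an arrow and damage the player.
; Death sets IsDead, stops movement, adjusts collision, reports the kill to ZombieGameMode and destroys the actor after a delay.
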(event OnSeePawn(PawnSensing)
  (params (Pawn :type Pawn%20Object%20Reference))
  ;[1 1 1] AI Perception
  (Utilities|Casting|CastToBP_FirstPersonCharacter Pawn)
  (Variables|/Script/Engine.CharacterMovementComponent|SetMaxWalkSpeed (Variables|Character|GetCharacterMovement) 3.6e+02)
  (AI|Components|Blackboard|SetValueasBool (AI|GetBlackboard 0) (Utilities|Name|MakeLiteralName "SeePlayer") true))

(event Custom|Death
  ;[0.7101 0.07196 0] Death
  (Variables|Default|SetIsDead true)
  (AI|Components|Blackboard|SetValueasBool (AI|GetBlackboard 0) (Utilities|Name|MakeLiteralName "IsDead") (Variables|Default|GetIsDead))
  (Variables|/Script/Engine.CharacterMovementComponent|SetMaxWalkSpeed (Variables|Character|GetCharacterMovement) 0.0)
  (Audio|Components|Audio|Stop (Variables|Default|GetHoarde))
  (Animation|PlayAnimMontage "/Game/_Main/Enemy/ZombieGirl/Animations/zombie_dying_Montage.zombie_dying_Montage" 1.0 "None")
  (Audio|PlaySoundatLocation "/Game/_Main/Sounds/Zombies/ZombieDeath.ZombieDeath" (Transformation|GetActorLocation) "0, 0, 0" 0.3 1.5 0.0 "/Game/MilitaryWeapSilver/Sound/Attenuation/WeaponShot_att.WeaponShot_att" 0 0 0)
  (Collision|SetCollisionEnabled (Variables|Collision|GetCapsuleComponent) "NoCollision")
  (Collision|SetCollisionEnabled (Variables|Character|GetMesh) "QueryOnly")
  (bind _aszombie_game_mode (Utilities|Casting|CastToZombieGameMode (Game|GetGameMode)))
  (Default|ZombieKilled _aszombie_game_mode)
  (bind _output_get (Variables|/Game/_Main/Blueprints/ZombieGameMode.ZombieGameMode_C|SetZombiesSpawned _aszombie_game_mode (Variables|/Game/_Main/Blueprints/ZombieGameMode.ZombieGameMode_C|GetZombiesSpawned _aszombie_game_mode)))
  (Utilities|Array|RemoveItem _output_get self)
  (Utilities|FlowControl|Delay 2e+01)
  (Actor|DestroyActor))

(event Custom|Attack
  ;[1 0.08801 0.9467] Attack
  (Animation|Montage|PlayMontage (Variables|Character|GetMesh) "/Game/_Main/Enemy/ZombieGirl/Animations/zombie_attack_Montage1.zombie_attack_Montage1"
    (:OnNotifyBegin
      (bind (_outactors _returnvalue) (Collision|SphereOverlapActors (Transformation|GetWorldLocation (Variables|Default|GetArrow1)) 8e+01 (Utilities|Array|MakeArray "ObjectTypeQuery3") "/Game/_Main/Blueprints/BP_FirstPersonCharacter.BP_FirstPersonCharacter_C" (Utilities|Array|MakeArray self)))
      (if _returnvalue
        (for _array_element _outactors
          (Game|Damage|ApplyDamage _array_element 2e+01 (Pawn|GetController) self "/Script/Engine.DamageType")
          (Audio|PlaySoundatLocation "/Game/_Main/Sounds/Zombies/Attack_ZombieGirl.Attack_ZombieGirl" (Transformation|GetActorLocation) "0, 0, 0" 0.3 1.0 0.0 "/Game/MilitaryWeapSilver/Sound/Attenuation/WeaponShot_att.WeaponShot_att" 0 0 0))))))

(event Game|Damage|EventPointDamage
  (params (Damage :type Float%20%28single-precision%29) (DamageType :type Damage%20Type%20Object%20Reference) (HitLocation :type Vector :default "0, 0, 0") (HitNormal :type Vector :default "0, 0, 0") (HitComponent :type Primitive%20Component%20Object%20Reference) (BoneName :type Name :default "None") (ShotFromDirection :type Vector :default "0, 0, 0") (InstigatedBy :type Controller%20Object%20Reference) (DamageCauser :type Actor%20Object%20Reference) (HitInfo :type Hit%20Result%20Structure%20%28by%20ref%29))
  ;[1 0.001736 0.1123] Take Damage
  (if (not (Variables|Default|GetIsDead))
    (if (<= (Variables|Default|GetHealth) 0.0)
      (CallFunction|Death)
      (else
        (bind _output_get (Variables|Default|SetHealth (- (Variables|Default|GetHealth) Damage)))
        (if (<= _output_get 0.0)
          (CallFunction|Death)
          (else
            (Animation|PlayAnimMontage "/Game/_Main/Enemy/ZombieGirl/Animations/Zombie_Reaction_Hit_mixamo_com_Montage.Zombie_Reaction_Hit_mixamo_com_Montage" 1.0 "None")
            (AI|Components|Blackboard|SetValueasBool (AI|GetBlackboard 0) (Utilities|Name|MakeLiteralName "SeePlayer") true)
            (Audio|PlaySoundatLocation "/Game/_Main/Sounds/Zombies/Attack_ZombieGirl.Attack_ZombieGirl" (Transformation|GetActorLocation) "0, 0, 0" 0.3 1.0 0.0 "/Game/MilitaryWeapSilver/Sound/Attenuation/WeaponShot_att.WeaponShot_att" 0 0 0)))))))

(fn ConstructionScript)