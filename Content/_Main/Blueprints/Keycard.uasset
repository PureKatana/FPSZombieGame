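; Keycard pickup that lets the player open the main gate.
; When BP_FirstPersonCharacter overlaps its box, it sets HasKeycard on the character, plays a checkpoint sound and shows an animated NotificationUI.
; After a short delay it removes the widget, destroys itself, then spawns a DialogueBox actor that starts the found-keycard dialogue and carries the next objective text.
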(event OnComponentBeginOverlap(Box)
  (params (OverlappedComponent :type Primitive%20Component%20Object%20Reference) (OtherActor :type Actor%20Object%20Reference) (OtherComp :type Primitive%20Component%20Object%20Reference) (OtherBodyIndex :type Integer) (bFromSweep :type Boolean) (SweepResult :type Hit%20Result%20Structure%20%28by%20ref%29))
  (bind _asbp_first_person_character (Utilities|Casting|CastToBP_FirstPersonCharacter OtherActor))
  (Variables|/Game/_Main/Blueprints/BP_FirstPersonCharacter.BP_FirstPersonCharacter_C|SetHasKeycard _asbp_first_person_character true)
  (Utilities|FlowControl|Sequence
    (:then_0
      (bind _returnvalue (UserInterface|CreateWidget "/Game/_Main/Images/UI_Widgets/NotificationUI.NotificationUI_C" (Game|GetPlayerController 0)))
      (bind _output_get (Variables|Default|SetNotifyUI _returnvalue))
      (UserInterface|Viewport|AddtoViewport _output_get 0)
      (Widget|SetVisibility (Variables|/Game/_Main/Images/UI_Widgets/NotificationUI.NotificationUI_C|GetTextBlock_0 (Variables|Default|GetNotifyUI)) "Hidden")
      (UserInterface|Animation|PlayAnimation (Variables|Default|GetNotifyUI) (Variables|/Game/_Main/Images/UI_Widgets/NotificationUI.NotificationUI_C|GetFade2 (Variables|Default|GetNotifyUI)) 0.0 1 "Forward" 1.0 false)
      (Audio|PlaySound2D "/Game/_Main/Sounds/SFX/Checkpoint.Checkpoint" 0.5 1.0 0.0 0 0))
    (:then_1
      (Utilities|FlowControl|Delay 2.0)
      (Widget|RemovefromParent (Variables|Default|GetNotifyUI))
      (Actor|DestroyActor)
      (bind _returnvalue_2 (Game|SpawnActorfromClass "/Game/_Main/Blueprints/DialogueBox.DialogueBox_C" (Math|Transform|MakeTransform "0, 0,-1100.000000") "Undefined" 0 (Utilities|Array|MakeArray "You : I found the keycard!" "You : I can go back and open the gate now!") "Activate the main gate." false 0))
      (Default|StartDialogue _returnvalue_2))))

(event EventBeginPlay)

(event Collision|EventActorBeginOverlap
  (params (OtherActor :type Actor%20Object%20Reference)))

(event EventTick
  (params (DeltaSeconds :type Float%20%28single-precision%29)))

(fn ConstructionScript)