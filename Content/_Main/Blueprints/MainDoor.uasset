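; Keycard-locked main door that slides along Z when the player opens it.
; A trigger box tracks the first-person character, enabling E input and showing a notification widget until the door has opened.
; With a keycard, E turns the keypad green and runs a one-time timeline opening, freezing walking until finished; CloseDoor reverses it.
; Without one, the widget fades with a denial sound, and the first attempt spawns dialogue setting a find-keycard objective.
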(event OnComponentBeginOverlap(Box)
  (params (OverlappedComponent :type Primitive%20Component%20Object%20Reference) (OtherActor :type Actor%20Object%20Reference) (OtherComp :type Primitive%20Component%20Object%20Reference) (OtherBodyIndex :type Integer) (bFromSweep :type Boolean) (SweepResult :type Hit%20Result%20Structure%20%28by%20ref%29))
  (Utilities|Casting|CastToBP_FirstPersonCharacter OtherActor)
  (Variables|Default|SetIsIn true)
  (if (not (Variables|Default|GetAlreadyOpened))
    (bind _returnvalue (UserInterface|CreateWidget "/Game/_Main/Images/UI_Widgets/NotificationUI.NotificationUI_C" (Game|GetPlayerController 0)))
    (bind _output_get (Variables|Default|SetNotifyUI _returnvalue))
    (UserInterface|Viewport|AddtoViewport _output_get 0)
    (Input|EnableInput (Game|GetPlayerController 0))))

(event OnComponentEndOverlap(Box)
  (params (OverlappedComponent :type Primitive%20Component%20Object%20Reference) (OtherActor :type Actor%20Object%20Reference) (OtherComp :type Primitive%20Component%20Object%20Reference) (OtherBodyIndex :type Integer))
  (Utilities|Casting|CastToBP_FirstPersonCharacter OtherActor)
  (Variables|Default|SetIsIn false)
  (Widget|RemovefromParent (Variables|Default|GetNotifyUI)))

(event Custom|CloseDoor
  (Audio|PlaySoundatLocation "/Game/_Main/Sounds/SFX/Open_CloseMainDoor.Open_CloseMainDoor" (Transformation|GetActorLocation) "0, 0, 0" 0.5 1.0 0.0 0 0 0 0)
  (bind _doorslide (Timeline|OpenDoor Reverse)
    (:Update
      (Transformation|SetRelativeLocation (Variables|Default|GetDoorUp) (Math|Vector|MakeVector 0.0 0.0 (* _doorslide 1.8e+02)) false false))
    (:Finished
      (Variables|/Script/Engine.CharacterMovementComponent|SetMaxWalkSpeed (Variables|/Script/Engine.Character|GetCharacterMovement (Game|GetPlayerCharacter 0)) 6e+02))))

(event Input|KeyboardEvents|E
  (params (Key :type Key%20Structure :default "None"))
  (bind _notifyui (Variables|Default|GetNotifyUI))
  (:Pressed
    (if (Variables|Default|GetIsIn)
      (bind _asbp_first_person_character (Utilities|Casting|CastToBP_FirstPersonCharacter (Game|GetPlayerCharacter 0)))
      (if (Variables|/Game/_Main/Blueprints/BP_FirstPersonCharacter.BP_FirstPersonCharacter_C|GetHasKeycard _asbp_first_person_character)
        (Variables|Default|SetAlreadyOpened true)
        (Utilities|FlowControl|DoOnce false
          (:Completed
            (Audio|PlaySoundatLocation "/Game/_Main/Sounds/SFX/UnlockDoor.UnlockDoor" (Transformation|GetActorLocation) "0, 0, 0" 0.5 0.2 0.0 0 0 0 0)
            (Audio|PlaySoundatLocation "/Game/_Main/Sounds/SFX/Open_CloseMainDoor.Open_CloseMainDoor" (Transformation|GetActorLocation) "0, 0, 0" 0.5 1.0 0.0 0 0 0 0)
            (Rendering|Material|SetMaterial (Variables|Default|GetKeypad) 0 "/Game/_Main/Maps/Materials/Green_Glow.Green_Glow")
            (Variables|/Script/Engine.CharacterMovementComponent|SetMaxWalkSpeed (Variables|/Script/Engine.Character|GetCharacterMovement (Game|GetPlayerCharacter 0)) 0.0)
            (bind _doorslide (Timeline|OpenDoor Play)
              (:Update
                (Transformation|SetRelativeLocation (Variables|Default|GetDoorUp) (Math|Vector|MakeVector 0.0 0.0 (* _doorslide 1.8e+02)) false false))
              (:Finished
                (Variables|/Script/Engine.CharacterMovementComponent|SetMaxWalkSpeed (Variables|/Script/Engine.Character|GetCharacterMovement (Game|GetPlayerCharacter 0)) 6e+02)))))
        (else
          (UserInterface|Animation|PlayAnimation _notifyui (Variables|/Game/_Main/Images/UI_Widgets/NotificationUI.NotificationUI_C|GetFade _notifyui) 0.0 1 "Forward" 1.0 false)
          (Audio|PlaySoundatLocation "/Game/_Main/Sounds/SFX/Select.Select" (Transformation|GetActorLocation) "0, 0, 0" 0.5 0.2 0.0 0 0 0 0)
          (Utilities|FlowControl|DoOnce false
            (:Completed
              (bind _asbp_first_person_character_2 (Utilities|Casting|CastToBP_FirstPersonCharacter (Game|GetPlayerCharacter 0)))
              (Variables|/Game/_Main/Blueprints/BP_FirstPersonCharacter.BP_FirstPersonCharacter_C|SetDoorInteract _asbp_first_person_character_2 true)
              (Utilities|FlowControl|Delay 1.0)
              (bind _returnvalue (Game|SpawnActorfromClass "/Game/_Main/Blueprints/DialogueBox.DialogueBox_C" (Math|Transform|MakeTransform "0, 0,-1000.000000") "Undefined" 0 (Utilities|Array|MakeArray "You : I need a keycard to open the gate." "You : It might be behind the door next to me.") "Find a keycard" false 0))
              (Default|StartDialogue _returnvalue))))))))

(fn ConstructionScript)