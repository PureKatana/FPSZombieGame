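; ElevatorManager is the interactable elevator that starts the zombie survival wave and rises once the game is won.
; A trigger box shows a prompt, and pressing E inside runs a DoOnce-guarded branch on the game mode's WinGame.
; Before winning, a delayed sequence plays boot-up sounds, red lights and dialogue, then starts the wave with music stopped later by dispatcher.
; After winning, a timeline lifts the elevator and turns Cube1 green.
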(event OnComponentBeginOverlap(Box)
  (params (OverlappedComponent :type Primitive%20Component%20Object%20Reference) (OtherActor :type Actor%20Object%20Reference) (OtherComp :type Primitive%20Component%20Object%20Reference) (OtherBodyIndex :type Integer) (bFromSweep :type Boolean) (SweepResult :type Hit%20Result%20Structure%20%28by%20ref%29))
  (Utilities|Casting|CastToBP_FirstPersonCharacter OtherActor)
  (Variables|Default|SetIsIn true)
  (if (not (Variables|Default|GetAlreadyPressed))
    (bind _returnvalue (UserInterface|CreateWidget "/Game/_Main/Images/UI_Widgets/NotificationUI.NotificationUI_C" (Game|GetPlayerController 0)))
    (bind _output_get (Variables|Default|SetNotifyUI _returnvalue))
    (UserInterface|Viewport|AddtoViewport _output_get 0)
    (Input|EnableInput (Game|GetPlayerController 0))))

(event OnComponentEndOverlap(Box)
  (params (OverlappedComponent :type Primitive%20Component%20Object%20Reference) (OtherActor :type Actor%20Object%20Reference) (OtherComp :type Primitive%20Component%20Object%20Reference) (OtherBodyIndex :type Integer))
  (Utilities|Casting|CastToBP_FirstPersonCharacter OtherActor)
  (Variables|Default|SetIsIn false)
  (Widget|RemovefromParent (Variables|Default|GetNotifyUI)))

(event Custom|StopMusic
  (Audio|Components|Audio|Stop (Variables|Default|GetIntenseMusic)))

(event Input|KeyboardEvents|E
  (params (Key :type Key%20Structure :default "None"))
  (:Pressed
    (if (Variables|Default|GetIsIn)
      (Utilities|Casting|CastToBP_FirstPersonCharacter (Game|GetPlayerCharacter 0))
      (Utilities|FlowControl|DoOnce false :!label _label
        (:Completed
          (if (Variables|/Game/_Main/Blueprints/ZombieGameMode.ZombieGameMode_C|GetWinGame (.AsZombie%20Game%20Mode (Utilities|Casting|CastToZombieGameMode (Game|GetGameMode))))
            (Audio|PlaySound2D "/Game/_Main/Sounds/SFX/UnlockDoor.UnlockDoor" 0.5 1.0 0.5 0 0)
            (Variables|Default|SetAlreadyPressed true)
            (bind _newtrack_0 (Timeline|MoveUp Play)
              (:Update
                (Transformation|SetRelativeLocation (Variables|Default|GetElevator) _newtrack_0 false false)
                (Rendering|Material|SetMaterial (Variables|Default|GetCube1) 0 "/Game/_Main/Maps/Materials/Green_Glow.Green_Glow")))
            (elif (not (Variables|Default|GetWaveStarted))
              (Default|CallStopMusicDispatcher (.AsZombie%20Game%20Mode (Utilities|Casting|CastToZombieGameMode (Game|GetGameMode))))
              (Audio|PlaySoundatLocation "/Game/_Main/Sounds/SFX/UnlockDoor.UnlockDoor" (Transformation|GetActorLocation) "0, 0, 0" 0.5 1.0 0.5 0 0 0 0)
              (Utilities|FlowControl|Delay 1.0)
              (Audio|PlaySoundatLocation "/Game/_Main/Sounds/SFX/EngineBooting.EngineBooting" (Transformation|GetActorLocation) "0, 0, 0" 0.5 1.0 0.0 0 0 0 0)
              (Utilities|FlowControl|Sequence
                (:then_0
                  (for _array_element (Variables|Default|GetLights)
                    (Rendering|Material|SetMaterial (Variables|/Script/Engine.StaticMeshActor|GetStaticMeshComponent _array_element) 0 "/Game/_Main/Maps/Materials/Red_Glow.Red_Glow"))
                  (bind _returnvalue (Game|SpawnActorfromClass "/Game/_Main/Blueprints/DialogueBox.DialogueBox_C" (Math|Transform|MakeTransform "0, 0, 0") "Undefined" 0 (Utilities|Array|MakeArray "You : The elevator is booting up." "You : It'll take a while for it to work properly.") "" false 0))
                  (Default|StartDialogue _returnvalue))
                (:then_1
                  (Utilities|FlowControl|Delay 8.0)
                  (Variables|/Script/Engine.CharacterMovementComponent|SetMaxWalkSpeed (Variables|/Script/Engine.Character|GetCharacterMovement (Game|GetPlayerCharacter 0)) 0.0)
                  (Audio|PlaySound2D "/Game/_Main/Sounds/SFX/ZombieHorde.ZombieHorde" 0.5 1.0 0.0 0 0)
                  (Utilities|FlowControl|Delay 6.0)
                  (bind _returnvalue_2 (Game|SpawnActorfromClass "/Game/_Main/Blueprints/DialogueBox.DialogueBox_C" (Math|Transform|MakeTransform "0, 0,1000.000000") "Undefined" 0 (Utilities|Array|MakeArray "You : Damn it! " "You : A lot of zombies are coming." "You : I have to survive until the elevator comes back up.") "Survive until the elevator is active." true 0))
                  (Default|StartDialogue _returnvalue_2)
                  (Utilities|FlowControl|Delay 12.0)
                  (bind _returnvalue_3 (Audio|SpawnSound2D "/Game/_Main/Sounds/Music/Intense.Intense" 0.3 1.0 0.0 0))
                  (Variables|Default|SetIntenseMusic _returnvalue_3)
                  (bind _aszombie_game_mode (Utilities|Casting|CastToZombieGameMode (Game|GetGameMode)))
                  (Default|StartWaveGame _aszombie_game_mode)
                  (Variables|Default|SetWaveStarted true)
                  (EventDispatchers|BindEventtoElevatorDispatcher _aszombie_game_mode (delegate Custom|StopMusic))
                  (goto _label Reset))))))))))

(fn ConstructionScript)