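; AmmoPickup is a pickup actor that gives ammo to the first-person player character when it overlaps the pickup's sphere.
; The overlap adds AmmoAmount to the character's total ammo and also refills the current clip to its maximum size.
; A DoOnce gate limits it to one use, then it plays a pickup sound and destroys itself after a short delay.
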(event OnComponentBeginOverlap(Sphere)
  (params (OverlappedComponent :type Primitive%20Component%20Object%20Reference) (OtherActor :type Actor%20Object%20Reference) (OtherComp :type Primitive%20Component%20Object%20Reference) (OtherBodyIndex :type Integer) (bFromSweep :type Boolean) (SweepResult :type Hit%20Result%20Structure%20%28by%20ref%29))
  (bind _asbp_first_person_character (Utilities|Casting|CastToBP_FirstPersonCharacter OtherActor))
  (Utilities|FlowControl|DoOnce false
    (:Completed
      (Variables|/Game/_Main/Blueprints/BP_FirstPersonCharacter.BP_FirstPersonCharacter_C|SetTotalAmmo _asbp_first_person_character (+ (Variables|/Game/_Main/Blueprints/BP_FirstPersonCharacter.BP_FirstPersonCharacter_C|GetTotalAmmo _asbp_first_person_character) (Variables|Default|GetAmmoAmount)))
      (Variables|/Game/_Main/Blueprints/BP_FirstPersonCharacter.BP_FirstPersonCharacter_C|SetCurrentAmmo _asbp_first_person_character (Variables|/Game/_Main/Blueprints/BP_FirstPersonCharacter.BP_FirstPersonCharacter_C|GetMaxClipSize _asbp_first_person_character))
      (Audio|PlaySound2D "/Game/MilitaryWeapSilver/Sound/Pistol/Wavs/Pistol_AmmoPickup.Pistol_AmmoPickup" 0.5 1.0 0.0 0 0)
      (Utilities|FlowControl|Delay 0.2)
      (Actor|DestroyActor))))

(fn ConstructionScript)