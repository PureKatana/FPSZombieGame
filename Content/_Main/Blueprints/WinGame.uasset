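; WinGame is a trigger actor that runs the win sequence when the first-person player character overlaps its box.
; The overlap disables the character's input, creates the WinUI widget and adds it to the viewport.
; Timed delays stage the widget's fades for black screen, text and buttons, with a 2D sound accompanying the text and the mouse cursor shown at the end.
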(event OnComponentBeginOverlap(Box)
  (params (OverlappedComponent :type Primitive%20Component%20Object%20Reference) (OtherActor :type Actor%20Object%20Reference) (OtherComp :type Primitive%20Component%20Object%20Reference) (OtherBodyIndex :type Integer) (bFromSweep :type Boolean) (SweepResult :type Hit%20Result%20Structure%20%28by%20ref%29))
  (bind _returnvalue (Game|GetPlayerController 0))
  (bind _asbp_first_person_character (Utilities|Casting|CastToBP_FirstPersonCharacter OtherActor))
  (Input|DisableInput _asbp_first_person_character _returnvalue)
  (bind _returnvalue_2 (UserInterface|CreateWidget "/Game/_Main/Images/UI_Widgets/WinUI.WinUI_C" _returnvalue))
  (bind _output_get (Variables|Default|SetWinUI _returnvalue_2))
  (UserInterface|Viewport|AddtoViewport _output_get 0)
  (UserInterface|Animation|PlayAnimation (Variables|Default|GetWinUI) (Variables|/Game/_Main/Images/UI_Widgets/WinUI.WinUI_C|GetFadeBlackScreen (Variables|Default|GetWinUI)) 0.0 1 "Forward" 1.0 false)
  (Utilities|FlowControl|Delay 6.0)
  (UserInterface|Animation|PlayAnimation (Variables|Default|GetWinUI) (Variables|/Game/_Main/Images/UI_Widgets/WinUI.WinUI_C|GetFadeText (Variables|Default|GetWinUI)) 0.0 1 "Forward" 1.0 false)
  (Audio|PlaySound2D "/Game/_Main/Sounds/SFX/Select.Select" 0.5 1.0 0.0 0 0)
  (Utilities|FlowControl|Delay 4.0)
  (UserInterface|Animation|PlayAnimation (Variables|Default|GetWinUI) (Variables|/Game/_Main/Images/UI_Widgets/WinUI.WinUI_C|GetFadeButtons (Variables|Default|GetWinUI)) 0.0 1 "Forward" 1.0 false)
  (Variables|/Script/Engine.PlayerController|SetbShowMouseCursor (Game|GetPlayerController 0) true))

(fn ConstructionScript)