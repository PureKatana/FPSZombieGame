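; DialogueBox is a one-shot trigger actor that plays a sequence of dialogue lines when the first-person player overlaps its box.
; A looping timer types each line into a widget character by character with sound, pausing before advancing to the next.
; FreezePlayer optionally zeroes walk speed during dialogue.
; Afterwards it removes the widget, shows any new objective on the player's objective UI, restores speed and later destroys itself.
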(event OnComponentBeginOverlap(Box)
  (params (OverlappedComponent :type Primitive%20Component%20Object%20Reference) (OtherActor :type Actor%20Object%20Reference) (OtherComp :type Primitive%20Component%20Object%20Reference) (OtherBodyIndex :type Integer) (bFromSweep :type Boolean) (SweepResult :type Hit%20Result%20Structure%20%28by%20ref%29))
  (Utilities|Casting|CastToBP_FirstPersonCharacter OtherActor)
  (Utilities|FlowControl|DoOnce false
    (:Completed
      (CallFunction|StartDialogue)
      (if (Variables|Default|GetFreezePlayer)
        (Variables|/Script/Engine.CharacterMovementComponent|SetMaxWalkSpeed (Variables|/Script/Engine.Character|GetCharacterMovement (stale Custom|StartDialogue _asbp_first_person_character)) 0.0)))))

(event Custom|StartDialogue
  (bind _asbp_first_person_character (Utilities|Casting|CastToBP_FirstPersonCharacter (Game|GetPlayerCharacter 0)))
  (Math|Integer|IncrementInt (Variables|Default|GetDialogueIndex)
    (:%20%20
      (if (< (Variables|Default|GetDialogueIndex) (Utilities|Array|Length (Variables|Default|GetDialogue)))
        (Variables|Default|GetDialogueUI
          (:then
            _)
          (:else
            (bind _returnvalue (UserInterface|CreateWidget "/Game/_Main/Images/UI_Widgets/DialogueUI.DialogueUI_C" (Game|GetPlayerController 0)))
            (bind _output_get (Variables|Default|SetDialogueUI _returnvalue))
            (UserInterface|Viewport|AddtoViewport _output_get 0)))
        (bind _returnvalue_2 (Utilities|Time|SetTimerbyEvent (delegate Custom|Set%20Text) (Variables|Default|GetSpeed) true))
        (else
          (Widget|RemovefromParent (Variables|Default|GetDialogueUI))
          (Utilities|FlowControl|Delay 1.0)
          (CallFunction|UpdateObjective)
          (Variables|Default|SetDialogueFinished true)
          (if (Variables|Default|GetFreezePlayer)
            (Variables|/Script/Engine.CharacterMovementComponent|SetMaxWalkSpeed (Variables|/Script/Engine.Character|GetCharacterMovement _asbp_first_person_character) 6e+02)))))))

(event Custom|UpdateObjective
  (bind _asbp_first_person_character (Utilities|Casting|CastToBP_FirstPersonCharacter (Game|GetPlayerCharacter 0)))
  (if (not (Utilities|Array|IsEmpty (Variables|Default|GetObjectiveText)))
    (Rendering|Components|TextRender|SetText (Variables|/Game/_Main/Images/UI_Widgets/ObjectiveUI.ObjectiveUI_C|GetObjective (Variables|/Game/_Main/Blueprints/BP_FirstPersonCharacter.BP_FirstPersonCharacter_C|GetObjUI _asbp_first_person_character)) (Utilities|Text|ToText(String) (Variables|Default|GetObjectiveText)))
    (UserInterface|Animation|PlayAnimation (Variables|/Game/_Main/Blueprints/BP_FirstPersonCharacter.BP_FirstPersonCharacter_C|GetObjUI _asbp_first_person_character) (Variables|/Game/_Main/Images/UI_Widgets/ObjectiveUI.ObjectiveUI_C|GetFadeObj (Variables|/Game/_Main/Blueprints/BP_FirstPersonCharacter.BP_FirstPersonCharacter_C|GetObjUI _asbp_first_person_character)) 0.0 1 "Forward" 1.0 false)
    (Audio|PlaySound2D "/Game/_Main/Sounds/SFX/Select.Select" 1.0 0.5 0.0 0 0)))

(event Custom|Set%20Text
  (bind _output_get (Variables|Default|SetDisplayText (Utilities|String|Append (Variables|Default|GetDisplayText) (Utilities|Array|Get(acopy) (Utilities|String|GetCharacterArrayfromString (Utilities|Array|Get(acopy) (Variables|Default|GetDialogue) (Variables|Default|GetDialogueIndex))) (Variables|Default|GetCharIndex)))))
  (Rendering|Components|TextRender|SetText (Variables|/Game/_Main/Images/UI_Widgets/DialogueUI.DialogueUI_C|GetDialogueText (Variables|Default|GetDialogueUI)) (Utilities|Text|ToText(String) _output_get))
  (Audio|PlaySound2D "/Game/_Main/Sounds/SFX/TextSound.TextSound" 0.5 1.2 0.0 0 0)
  (bind _result (Math|Integer|IncrementInt (Variables|Default|GetCharIndex))
    (:%20%20
      (if (== _result (Utilities|Array|Length (Utilities|String|GetCharacterArrayfromString (Utilities|Array|Get(acopy) (Variables|Default|GetDialogue) (Variables|Default|GetDialogueIndex)))))
        (Utilities|Time|ClearandInvalidateTimerbyHandle (stale _returnvalue_2))
        (Variables|Default|SetDisplayText "")
        (Variables|Default|SetCharIndex 0)
        (Audio|PlaySound2D "/Game/_Main/Sounds/SFX/Select.Select" 0.5 1.0 0.0 0 0)
        (Utilities|FlowControl|Delay 2.0)
        (Math|Integer|IncrementInt (Variables|Default|GetDialogueIndex)
          (:%20%20
            (if (< (Variables|Default|GetDialogueIndex) (Utilities|Array|Length (Variables|Default|GetDialogue)))
              (Variables|Default|GetDialogueUI
                (:then
                  _)
                (:else
                  (bind _returnvalue (UserInterface|CreateWidget "/Game/_Main/Images/UI_Widgets/DialogueUI.DialogueUI_C" (Game|GetPlayerController 0)))
                  (bind _output_get_2 (Variables|Default|SetDialogueUI _returnvalue))
                  (UserInterface|Viewport|AddtoViewport _output_get_2 0)))
              (bind _returnvalue_2 (Utilities|Time|SetTimerbyEvent (delegate Custom|Set%20Text) (Variables|Default|GetSpeed) true))
              (else
                (Widget|RemovefromParent (Variables|Default|GetDialogueUI))
                (Utilities|FlowControl|Delay 1.0)
                (CallFunction|UpdateObjective)
                (Variables|Default|SetDialogueFinished true)
                (if (Variables|Default|GetFreezePlayer)
                  (Variables|/Script/Engine.CharacterMovementComponent|SetMaxWalkSpeed (Variables|/Script/Engine.Character|GetCharacterMovement (stale Custom|StartDialogue _asbp_first_person_character)) 6e+02))))))))))

(event EventTick
  (params (DeltaSeconds :type Float%20%28single-precision%29))
  (if (Variables|Default|GetDialogueFinished)
    (Utilities|FlowControl|DoOnce false
      (:Completed
        (Utilities|FlowControl|Delay 5.0)
        (Actor|DestroyActor)))))

(fn ConstructionScript)