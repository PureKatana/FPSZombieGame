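; Sliding door actor that opens automatically when a first-person character with DoorInteract set enters its trigger box.
; On overlap it turns the indicator mesh to a green glow, plays the open sound and runs a timeline that slides the door mesh along X.
; Leaving the box, if the flag is still set, switches the glow to red, plays the close sound and reverses the timeline.
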(event OnComponentBeginOverlap(Box)
  (params (OverlappedComponent :type Primitive%20Component%20Object%20Reference) (OtherActor :type Actor%20Object%20Reference) (OtherComp :type Primitive%20Component%20Object%20Reference) (OtherBodyIndex :type Integer) (bFromSweep :type Boolean) (SweepResult :type Hit%20Result%20Structure%20%28by%20ref%29))
  (bind _asbp_first_person_character (Utilities|Casting|CastToBP_FirstPersonCharacter OtherActor))
  (if (Variables|/Game/_Main/Blueprints/BP_FirstPersonCharacter.BP_FirstPersonCharacter_C|GetDoorInteract _asbp_first_person_character)
    (Rendering|Material|SetMaterial (Variables|Default|GetCube1) 0 "/Game/_Main/Maps/Materials/Green_Glow.Green_Glow")
    (Audio|PlaySoundatLocation "/Game/_Main/Sounds/SFX/OpenDoor.OpenDoor" (Transformation|GetActorLocation) "0, 0, 0" 0.5 1.0 0.0 0 0 0 0)
    (bind _newtrack_1 (Timeline|OpenDoor Play)
      (:Update
        (Transformation|SetRelativeLocation (Variables|Default|GetCube) (Math|Vector|MakeVector (* _newtrack_1 -2e+02) 0.0 0.0) false false)))))

(event OnComponentEndOverlap(Box)
  (params (OverlappedComponent :type Primitive%20Component%20Object%20Reference) (OtherActor :type Actor%20Object%20Reference) (OtherComp :type Primitive%20Component%20Object%20Reference) (OtherBodyIndex :type Integer))
  (bind _asbp_first_person_character (Utilities|Casting|CastToBP_FirstPersonCharacter OtherActor))
  (if (Variables|/Game/_Main/Blueprints/BP_FirstPersonCharacter.BP_FirstPersonCharacter_C|GetDoorInteract _asbp_first_person_character)
    (Rendering|Material|SetMaterial (Variables|Default|GetCube1) 0 "/Game/_Main/Maps/Materials/Red_Glow.Red_Glow")
    (Audio|PlaySoundatLocation "/Game/_Main/Sounds/SFX/CloseDoor.CloseDoor" (Transformation|GetActorLocation) "0, 0, 0" 0.5 1.0 0.0 0 0 0 0)
    (bind _newtrack_1 (Timeline|OpenDoor Reverse)
      (:Update
        (Transformation|SetRelativeLocation (Variables|Default|GetCube) (Math|Vector|MakeVector (* _newtrack_1 -2e+02) 0.0 0.0) false false)))))

(fn ConstructionScript)